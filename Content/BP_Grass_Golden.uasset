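; BP_Grass_Golden is a golden grass actor that is destroyed when an actor tagged Player overlaps it.
; The construction script creates a dynamic instance of the Grass_Gold material on the GrassG component and stores it in RandomGrassColour.
; On BeginPlay, it sets that instance's GrassColour parameter to a fixed gold with a randomised alpha, varying each clump.
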(event `self.ReceiveBeginPlay`
  ;[1 1 1] Changes grass colour
  (`MaterialInstanceDynamic.SetVectorParameterValue` (`self.RandomGrassColour`) "GrassColour" (`KismetMathLibrary.MakeColor` 1.0 0.8 0.08 (`KismetMathLibrary.RandomFloatInRange` 0.8 1.0))))

(event `self.GrassG.OnComponentBeginOverlap`
  (params (OverlappedComponent :type "PrimitiveComponent Object Reference") (OtherActor :type "Actor Object Reference") (OtherComp :type "PrimitiveComponent Object Reference") (OtherBodyIndex :type Integer) (bFromSweep :type Boolean) (SweepResult :type "HitResult Structure (by ref)"))
  ;[1 1 1] Breaks grass
  (if (`self.ActorHasTag` OtherActor "Player")
    (`self.K2_DestroyActor`)))

(fn `UserConstructionScript`
  (bind _returnvalue (`PrimitiveComponent.CreateDynamicMaterialInstance` (`self.GrassG`) 0 "/Game/Models/Grass/Grass_Gold.Grass_Gold" "Grass_Colour"))
  (set `self.RandomGrassColour` _returnvalue))